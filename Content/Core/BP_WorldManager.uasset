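; World manager actor that builds a blocky, Minecraft-style world out of block components added to itself.
; The Generate event prints the Vertices count, calls GenerateWorld, then walks each vertex, turning its offset height into a column of blocks stacked at fixed vertical steps.
; Each block goes through SpawnBlock, which adds an McBlock component at the given relative location.
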(event Custom|Generate
  (bind _vertices (Variables|Default|GetVertices))
  (Development|PrintString (Utilities|String|ToString(Integer) (Utilities|Array|Length _vertices)))
  (Class|McWorldManager|GenerateWorld 50)
  (for _array_element _vertices
    (for _index (range 0 (/ (Math|Float|Truncate (+ (.Z (Math|Vector|BreakVector _array_element)) 1.6e+03)) 100))
      (CallFunction|SpawnBlock (Math|Vector|MakeVector (.X (Math|Vector|BreakVector _array_element)) (.Y (Math|Vector|BreakVector _array_element)) (* _index 1e+02))))))

(event Custom|SpawnBlock
  (params (NewParam :type Vector))
  (AddComponent|AddMcBlockComponent false (Math|Transform|MakeTransform (Math|Vector|MakeVector (.x NewParam) (.y NewParam) (.z NewParam)) "0, 0, 0" "1,1,1")))

(event EventBeginPlay)

(event Collision|EventActorBeginOverlap
  (params (OtherActor :type Actor%20Object%20Reference)))

(event EventTick
  (params (DeltaSeconds :type Float%20%28single-precision%29)))

(fn ConstructionScript)