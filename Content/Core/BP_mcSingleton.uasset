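; BP_mcSingleton is a shared lookup point for the game's block assets and data.
; It supplies SM_BasicBlock as the default mesh and picks a default material by whether the block is player-placed, using the variations instance for blocks that are not.
; Block data comes from the DDT_Blocks data table, with the numeric ID converted to a row name.
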(fn GetDefaultMesh
  (return "/Game/Meshes/SM_BasicBlock.SM_BasicBlock"))

(fn GetBlockData
  (params (ID :type Byte :default 0))
  (bind _returnvalue (Utilities|GetDataTableRow "/Game/Data/DDT_Blocks.DDT_Blocks" (Utilities|String|StringToName (Utilities|String|ToString(Integer) (Math|Conversions|ToInteger(Byte) ID))))
    (:then
      (return _returnvalue))
    (:RowNotFound
      (return ""))))

(fn GetDefaultMaterial
  (params (PlayerPlaced :type Boolean))
  (return (select PlayerPlaced "/Game/Materials/M_BasicBlock.M_BasicBlock" "/Game/Materials/M_BasicBlock_Variations_Inst.M_BasicBlock_Variations_Inst")))