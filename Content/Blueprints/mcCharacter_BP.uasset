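; Player character Blueprint that shows the main game widget and animates a held pick tool.
; On BeginPlay it waits briefly for the world underneath to spawn, then turns on gravity and actor tick.
; After running the parent Tick, it swings PickHelper with a DoOnce-gated timeline while CurrentIntBlock is valid.
; Tick also toggles the tool mesh so it is hidden in placement mode.
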(event EventTick
  (params (DeltaSeconds :type Float%20%28single-precision%29))
  (|CallParentFunction DeltaSeconds)
  (Utilities|FlowControl|Sequence
    (:then_0
      ;[1 1 1] Simple Tool Anim
      (Utilities|IsValid (Variables|Default|GetCurrentIntBlock)
        (:Is%20Valid
          (Utilities|FlowControl|DoOnce false :!label _label
            (:Completed
              (bind _alpha (Timeline|PickAnim PlayFromStart)
                (:Update
                  (Transformation|SetRelativeRotation (Variables|Default|GetPickHelper) (Math|Rotator|MakeRotator 0.0 (* _alpha -6e+01) 0.0) false false))
                (:Finished
                  (Utilities|FlowControl|Sequence
                    (:then_0
                      (goto _label_2 Reset))
                    (:then_1
                      (goto _label Reset))))))))
        (:Is%20Not%20Valid
          (Utilities|FlowControl|DoOnce false :!label _label_2
            (:Completed
              (Utilities|FlowControl|Sequence
                (:then_0
                  (Timeline|PickAnim Stop))
                (:then_1
                  (Timeline|PickAnim SetNewTime))
                (:then_2
                  (goto _label Reset))))))))
    (:then_1
      ;[1 1 1] Hide Tool In Placement Mode
      (if (Math|Boolean|Equal(Boolean) (Variables|Default|GetbPlacementMode) (Rendering|IsVisible (Variables|Default|GetStaticMesh)))
        (Rendering|ToggleVisibility (Variables|Default|GetStaticMesh) false)))))

(event EventBeginPlay
  ;[1 1 1] Show Basic Onscreen Widget
  (bind _returnvalue (UserInterface|CreateWidget "/Game/UI/MainGame_Widget.MainGame_Widget_C"))
  (UserInterface|Viewport|AddtoViewport _returnvalue 0)
  ;[1 1 1] let the world underneath us spawn
  (Utilities|FlowControl|Delay 2.0)
  (Variables|/Script/Engine.CharacterMovementComponent|SetGravityScale (Variables|Character|GetCharacterMovement) 1.0)
  (Actor|Tick|SetActorTickEnabled true))

(fn ConstructionScript)